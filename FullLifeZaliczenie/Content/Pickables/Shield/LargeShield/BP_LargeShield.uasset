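; BP_LargeShield is a shield pickup that boosts the first-person character's ShieldCurrent when overlapped.
; The PickUpRange overlap passes a DoOnce before the character cast, so a failed cast leaves the gate closed.
; Below the full threshold it adds a fixed amount without clamping, plays a sound, prints a message and destroys itself.
; At full shield it prints a notice and reopens the gate after a delay.
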(event OnComponentBeginOverlap(PickUpRange)
  (params (OverlappedComponent :type Primitive%20Component%20Object%20Reference) (OtherActor :type Actor%20Object%20Reference) (OtherComp :type Primitive%20Component%20Object%20Reference) (OtherBodyIndex :type Integer) (bFromSweep :type Boolean) (SweepResult :type Hit%20Result%20Structure%20%28by%20ref%29))
  (Utilities|FlowControl|DoOnce false :!label _label
    (:Completed
      (bind _asbp_first_person_character (Utilities|Casting|CastToBP_FirstPersonCharacter OtherActor))
      (if (>= (Variables|/Game/FirstPerson/Blueprints/BP_FirstPersonCharacter.BP_FirstPersonCharacter_C|GetShieldCurrent _asbp_first_person_character) 1e+02)
        (Development|PrintString "Your shield is full.")
        (Utilities|FlowControl|Delay 3.5)
        (goto _label Reset)
        (else
          (Audio|PlaySoundatLocation "/Game/Pickables/Medkit/Sound/health_pickup22_.health_pickup22_" "0, 0, 0" "0, 0, 0" 0.8 1.0 0.0 0 0 0 0)
          (Variables|/Game/FirstPerson/Blueprints/BP_FirstPersonCharacter.BP_FirstPersonCharacter_C|SetShieldCurrent _asbp_first_person_character (+ (Variables|/Game/FirstPerson/Blueprints/BP_FirstPersonCharacter.BP_FirstPersonCharacter_C|GetShieldCurrent _asbp_first_person_character) 1e+02))
          (Development|PrintString "You've found large shield.")
          (Actor|DestroyActor))))))

(fn ConstructionScript)