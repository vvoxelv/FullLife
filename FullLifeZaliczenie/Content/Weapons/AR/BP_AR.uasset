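; Pickable assault rifle for the first-person character, setting its mesh from a weapon data table.
; Overlapping grants the rifle and enables input; dropping writes combined AR ammo to the pistol reserve and spawns a fresh BP_AR.
; A gate and retriggerable delay loop drives automatic fire, with ammo checks, debug-drawn traces whose hits go unused, sound and recoil.
; Reloading refills the magazine from the player's reserve after a timeline animation.
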(event OnComponentBeginOverlap(PickupRange)
  (params (OverlappedComponent :type Primitive%20Component%20Object%20Reference) (OtherActor :type Actor%20Object%20Reference) (OtherComp :type Primitive%20Component%20Object%20Reference) (OtherBodyIndex :type Integer) (bFromSweep :type Boolean) (SweepResult :type Hit%20Result%20Structure%20%28by%20ref%29))
  ;[0.2708 0.446 1] Pickable
  (bind _asbp_first_person_character (Utilities|Casting|CastToBP_FirstPersonCharacter OtherActor))
  (bind _output_get (Variables|Default|SetPlayer_Ref _asbp_first_person_character))
  (if (not (Variables|/Game/FirstPerson/Blueprints/BP_FirstPersonCharacter.BP_FirstPersonCharacter_C|GetbHasAR (Variables|Default|GetPlayer_Ref)))
    (Variables|/Game/FirstPerson/Blueprints/BP_FirstPersonCharacter.BP_FirstPersonCharacter_C|SetbHasAR _output_get true)
    (Input|EnableInput (Game|GetPlayerController 0))
    (Audio|PlaySoundatLocation "/Game/Weapons/PickableEffects/Gun_Pickup.Gun_Pickup" "0, 0, 0" "0, 0, 0" 1.5 0.8 0.0 0 0 0 0)
    (Components|DestroyComponent (Variables|Default|GetPickupRange))))

(event Input|EnhancedActionEvents|EnhancedInputActionIA_Shoot
  (params (ActionValue :type Boolean) (ElapsedSeconds :type Float%20%28double-precision%29) (TriggeredSeconds :type Float%20%28double-precision%29) (InputAction :type Input%20Action%20Object%20Reference :default "/Game/FirstPerson/Input/Actions/IA_Shoot.IA_Shoot"))
  (bind (_returnvalue _returnvalue2) (|PlayerPosition))
  ;[1 0.5097 0 1 25] Shooting
  (:Started
    (|AutomaticWeapon :!label _label
      (:then_0
        (|Weapon/Reloading/Ammo/Equipped?)
        (bind _outhit (Collision|LineTraceByChannel _returnvalue _returnvalue2 "TraceTypeQuery1" false 0 "ForDuration"))
        (Audio|PlaySoundatLocation "/Game/Weapons/AR/Sound/AR_Shoot.AR_Shoot" "0, 0, 0" "0, 0, 0" 1.0 1.0 0.0 0 0 0 0)
        (Variables|Default|SetAR_CurrentAmmo (- (Variables|Default|GetAR_CurrentAmmo) 1.0))
        (|ShootingAnimation)
        (Default|MuzzleFlashAR (Variables|Default|GetPlayer_Ref)))))
  (:Completed
    (goto _label Close)))

(event Input|EnhancedActionEvents|EnhancedInputActionIA_DropWeapon
  (params (ActionValue :type Boolean) (ElapsedSeconds :type Float%20%28double-precision%29) (TriggeredSeconds :type Float%20%28double-precision%29) (InputAction :type Input%20Action%20Object%20Reference :default "/Game/FirstPerson/Input/Actions/IA_DropWeapon.IA_DropWeapon"))
  (bind _player_ref (Variables|Default|GetPlayer_Ref))
  (bind _player_ref_2 (Variables|Default|GetPlayer_Ref))
  (bind _player_ref_3 (Variables|Default|GetPlayer_Ref))
  (bind _weapondroparrow (Variables|/Game/FirstPerson/Blueprints/BP_FirstPersonCharacter.BP_FirstPersonCharacter_C|GetWeaponDropArrow _player_ref_3))
  (bind _returnvalue (Transformation|GetWorldTransform _weapondroparrow))
  ;[1 1 1 1 24] WeaponDrop
  (:Started
    (if (Variables|/Game/FirstPerson/Blueprints/BP_FirstPersonCharacter.BP_FirstPersonCharacter_C|GetbHasAR (Variables|Default|GetPlayer_Ref))
      (if (Variables|/Game/FirstPerson/Blueprints/BP_FirstPersonCharacter.BP_FirstPersonCharacter_C|Get1WeaponEquipped (Variables|Default|GetPlayer_Ref))
        (Variables|/Game/FirstPerson/Blueprints/BP_FirstPersonCharacter.BP_FirstPersonCharacter_C|SetP_PistolReserveCurrent _player_ref (+ (Variables|Default|GetAR_CurrentAmmo) (Variables|/Game/FirstPerson/Blueprints/BP_FirstPersonCharacter.BP_FirstPersonCharacter_C|GetP_ARReserveCurrent _player_ref)))
        (Variables|/Game/FirstPerson/Blueprints/BP_FirstPersonCharacter.BP_FirstPersonCharacter_C|SetbHasAR _player_ref_2 false)
        (Rendering|SetVisibility (Variables|/Game/FirstPerson/Blueprints/BP_FirstPersonCharacter.BP_FirstPersonCharacter_C|GetPlayerAR _player_ref_2) false false)
        (Input|DisableInput (Game|GetPlayerController 0))
        (Actor|DestroyActor)
        (Game|SpawnActorfromClass "BP_AR_C" (Math|Transform|MakeTransform (.location _returnvalue) (.rotation _returnvalue) "1.000000,1.000000,1.000000") "AdjustIfPossibleButAlwaysSpawn" 0 0)))))

(event Input|EnhancedActionEvents|EnhancedInputActionIA_Debug
  (params (ActionValue :type Boolean) (ElapsedSeconds :type Float%20%28double-precision%29) (TriggeredSeconds :type Float%20%28double-precision%29) (InputAction :type Input%20Action%20Object%20Reference :default "/Game/FirstPerson/Input/Actions/IA_Debug.IA_Debug"))
  ;[0.2031 0 0.1715] DEBUG
  (:Started
    (Development|PrintString (Utilities|String|ToString(Float) (Variables|Default|GetAR_MagSize)) true true "(R=1.000000,G=0.000000,B=0.023286,A=1.000000)")
    (Development|PrintString (Utilities|String|ToString(Float) (Variables|Default|GetAR_CurrentAmmo)) true true "(R=1.000000,G=0.905640,B=0.000000,A=1.000000)")
    (Development|PrintString (Utilities|String|ToString(Float) (Variables|/Game/FirstPerson/Blueprints/BP_FirstPersonCharacter.BP_FirstPersonCharacter_C|GetP_ARReserveCurrent (Variables|Default|GetPlayer_Ref))))))

(event Input|EnhancedActionEvents|EnhancedInputActionIA_Reload
  (params (ActionValue :type Boolean) (ElapsedSeconds :type Float%20%28double-precision%29) (TriggeredSeconds :type Float%20%28double-precision%29) (InputAction :type Input%20Action%20Object%20Reference :default "/Game/FirstPerson/Input/Actions/IA_Reload.IA_Reload"))
  ;[0 0.9622 1 1 25] Reloading
  (:Started
    (if (Variables|/Game/FirstPerson/Blueprints/BP_FirstPersonCharacter.BP_FirstPersonCharacter_C|Get1WeaponEquipped (Variables|Default|GetPlayer_Ref))
      (|IsCurrentAmmo=MaxMagAmmo?
        (:If%20Not
          (|PlayerGotAnyAmmoToReload?
            (:Yes
              (Audio|PlaySoundatLocation "/Game/Weapons/AR/Sound/AR_Reload.AR_Reload" "0, 0, 0" "0, 0, 0" 1.0 1.0 0.0 0 0 0 0)
              (Variables|/Game/FirstPerson/Blueprints/BP_FirstPersonCharacter.BP_FirstPersonCharacter_C|SetIsReloading? (Variables|Default|GetPlayer_Ref) true)
              (|ReloadAnimation
                (:Finished
                  (|RELOADLOGIC)
                  (if (< (Variables|/Game/FirstPerson/Blueprints/BP_FirstPersonCharacter.BP_FirstPersonCharacter_C|GetP_ARReserveCurrent (Variables|Default|GetPlayer_Ref)) 0.0)
                    (Variables|/Game/FirstPerson/Blueprints/BP_FirstPersonCharacter.BP_FirstPersonCharacter_C|SetP_ARReserveCurrent (Variables|Default|GetPlayer_Ref) 0.0))
                  (Variables|/Game/FirstPerson/Blueprints/BP_FirstPersonCharacter.BP_FirstPersonCharacter_C|SetIsReloading? (Variables|Default|GetPlayer_Ref) false))))))))))

(event EventBeginPlay
  (bind _returnvalue (Utilities|GetDataTableRow (Variables|Default|GetWeaponDataBase) (Utilities|String|StringToName (Utilities|String|EnumtoString (Variables|Default|GetWeaponType))))
    (:then
      (Components|StaticMesh|SetStaticMesh (Variables|Default|GetARFull_Mesh) (.WeaponMesh (Utilities|Struct|BreakWeaponParameters _returnvalue))))))

(fn ConstructionScript)