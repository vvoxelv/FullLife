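; Sniper rifle weapon drop pickup that gives the first-person character a weapon when overlapped.
; On BeginPlay it looks up its weapon type in a data table to set the type, slot and displayed mesh.
; On overlap it checks the player's slot map and, only if that slot holds Hands, adds the weapon, destroys itself and plays a pickup sound.
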(event Collision|EventActorBeginOverlap
  (params (OtherActor :type Actor%20Object%20Reference))
  (bind _asbp_first_person_character (Utilities|Casting|CastToBP_FirstPersonCharacter OtherActor))
  (bind _output_get (Variables|Default|SetPlayer_Ref _asbp_first_person_character))
  (switch Utilities|FlowControl|Switch|SwitchonWeaponSlot (Variables|Default|GetWeaponSlot)
    (:NewEnumerator0
      _)
    (:NewEnumerator1
      _))
  (switch Utilities|FlowControl|Switch|SwitchonWeaponType (.Value (Utilities|Map|Find (Variables|/Game/FirstPerson/Blueprints/BP_FirstPersonCharacter.BP_FirstPersonCharacter_C|GetWeaponSlotMap (Variables|Default|GetPlayer_Ref)) (Variables|Default|GetWeaponSlot)))
    (:NewEnumerator4
      (Default|AddNewWeapon _output_get (Variables|Default|GetWeaponSlot) (Variables|Default|GetWeapon%20Type))
      (Actor|DestroyActor)
      (Audio|PlaySoundatLocation "/Game/Weapons/PickableEffects/getgun01b_22.getgun01b_22" "0, 0, 0" "0, 0, 0" 1.2 0.8 0.0 0 0 0 0))))

(event EventBeginPlay
  (bind _returnvalue (Utilities|GetDataTableRow (Variables|Default|GetWeapon%20Data%20Base) (Utilities|String|StringToName (Utilities|String|EnumtoString (Variables|Default|GetWeaponType))))
    (:then
      (Variables|Default|SetWeapon%20Type (.WeaponType (Utilities|Struct|BreakWeaponParameters _returnvalue)))
      (Variables|Default|SetWeaponSlot (.WeaponSlot (Utilities|Struct|BreakWeaponParameters _returnvalue)))
      (Components|StaticMesh|SetStaticMesh (Variables|Default|GetWeapon) (.WeaponMesh (Utilities|Struct|BreakWeaponParameters _returnvalue))))))

(fn ConstructionScript)