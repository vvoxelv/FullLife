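; BP_AICorpse is a corpse enemy that patrols between two waypoints and attacks the first-person player on sight.
; Tick drives delayed AIMoveTo patrols while no player is seen, flip-flopping the waypoint on arrival.
; PawnSensing triggers a chase ending in an attack animation and damage, with a retriggerable delay clearing the sighting flag.
; Animations play directly on the mesh, and incoming damage reduces health until the actor is destroyed.
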(event OnSeePawn(PawnSensing)
  (params (Pawn :type Pawn%20Object%20Reference))
  (bind _mesh (Variables|Character|GetMesh))
  (bind _asbp_first_person_character (Utilities|Casting|CastToBP_FirstPersonCharacter Pawn))
  (Utilities|FlowControl|Sequence
    (:then_0
      (Variables|Default|SetcanSeeEnemy true)
      (Utilities|FlowControl|Delay 0.4)
      (AI|AIMoveTo self "0, 0, 0" _asbp_first_person_character 5.0 false
        (:then
          (Components|Animation|PlayAnimation _mesh "/Game/CityofBrass_Enemies/Meshes/Enemy/Corpse/animation/Corpse_Run_Forward.Corpse_Run_Forward" true))
        (:OnSuccess
          (Components|Animation|PlayAnimation _mesh "/Game/CityofBrass_Enemies/Meshes/Enemy/Corpse/animation/Corpse_Alert_Attack_Basic01.Corpse_Alert_Attack_Basic01" false)
          (Game|Damage|ApplyDamage _asbp_first_person_character 1e+01 0 self))))
    (:then_1
      (Utilities|FlowControl|RetriggerableDelay 0.5)
      (Variables|Default|SetcanSeeEnemy false))))

(event EventBeginPlay
  (Variables|Default|SetWaypoint (Variables|Default|GetWaypoint1))
  (Variables|Default|SetHealthCurrent (Variables|Default|GetHealthMax)))

(event Collision|EventActorBeginOverlap
  (params (OtherActor :type Actor%20Object%20Reference)))

(event EventTick
  (params (DeltaSeconds :type Float%20%28single-precision%29))
  (bind _mesh (Variables|Character|GetMesh))
  (if (not (Variables|Default|GetcanSeeEnemy))
    (Utilities|FlowControl|Delay (Math|Random|RandomFloatinRange 2.0 5.0))
    (AI|AIMoveTo self (Transformation|GetWorldLocation (Variables|Default|GetWaypoint)) 0 5.0 false
      (:then
        (Components|Animation|PlayAnimation _mesh "/Game/CityofBrass_Enemies/Meshes/Enemy/Corpse/animation/Corpse_Run_Forward.Corpse_Run_Forward" true))
      (:OnSuccess
        (Components|Animation|PlayAnimation _mesh "/Game/CityofBrass_Enemies/Meshes/Enemy/Corpse/animation/Corpse_passive_idle.Corpse_passive_idle" true)
        (Utilities|FlowControl|FlipFlop
          (:A
            (Variables|Default|SetWaypoint (Variables|Default|GetWaypoint2)))
          (:B
            (Variables|Default|SetWaypoint (Variables|Default|GetWaypoint1))))))))

(event Game|Damage|EventAnyDamage
  (params (Damage :type Float%20%28single-precision%29) (DamageType :type Damage%20Type%20Object%20Reference) (InstigatedBy :type Controller%20Object%20Reference) (DamageCauser :type Actor%20Object%20Reference))
  (Variables|Default|SetHealthCurrent (- (Variables|Default|GetHealthCurrent) Damage))
  (if (not (> (Variables|Default|GetHealthCurrent) 0.0))
    (Actor|DestroyActor self)))

(fn ConstructionScript)